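; Boat helm actor that lets interaction steer the parent boat left or right in steps.
; Left and right interact events nudge a clamped helm position, call the helm update and play a click sound at the actor.
; The update event passes the position to the parent Actor_Boat through SetHelm.
; Tick rotates the helm mesh to match the current position.
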(event `self.Interact_Left`
  (set `self.HelmPosition` (`KismetMathLibrary.FClamp` (- (`self.HelmPosition`) 0.1) -1.0))
  (`self.Update_Helm` :!label _label)
  (`self.PlaySound`))

(event `self.Interact_Right`
  (set `self.HelmPosition` (`KismetMathLibrary.FClamp` (+ (`self.HelmPosition`) 0.1) -1.0))
  (goto _label))

(event `self.ReceiveTick`
  (params (DeltaSeconds :type "Float (single-precision)"))
  (`SceneComponent.K2_SetRelativeRotation` (`self.StaticMesh1`) (`KismetMathLibrary.MakeRotator` 0.0 (* (`self.HelmPosition`) -90.0) 90.0) false false))

(event `Update_Helm`
  (bind _asactor_boat (cast `Actor_Boat` (`self.GetParentActor`)))
  (`Actor_Boat.setHelm` _asactor_boat (`self.HelmPosition`)))

(event `PlaySound`
  (`GameplayStatics.PlaySoundAtLocation` "/Engine/VREditor/Sounds/UI/Gizmo_Handle_Clicked.Gizmo_Handle_Clicked" (`self.K2_GetActorLocation`) (struct) 1.0 1.0 0.0 "/Game/Blueprints/Attune_Generic.Attune_Generic" null null))

(fn `UserConstructionScript`)