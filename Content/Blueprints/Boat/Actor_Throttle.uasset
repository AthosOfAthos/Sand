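; Boat throttle lever actor that players step up or down with interact events.
; Each step clamps ThrottleVal between zero and one, calls UpdateBoat and plays a switch sound pitched by the value.
; Tick slides the lever mesh vertically to match the value.
; UpdateBoat casts the parent actor to Actor_Boat, but its SetThrottle call is unwired, so the value never reaches the boat.
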(event `self.Interact_Use`)

(event `PlaySound`
  (`GameplayStatics.PlaySoundAtLocation` "/Engine/VREditor/Sounds/UI/Flashlight_Switch.Flashlight_Switch" (`self.K2_GetActorLocation`) (struct) 1.0 (+ 0.8 (/ (`self.ThrottleVal`) 4.0)) 0.0 "/Game/Blueprints/Attune_Generic.Attune_Generic" null null))

(event `self.Interact_Up`
  (set `self.ThrottleVal` (`KismetMathLibrary.FClamp` (+ (`self.ThrottleVal`) (`self.StepAmmount`))))
  (`self.UpdateBoat` :!label _label)
  (`self.PlaySound`))

(event `self.ReceiveTick`
  (params (DeltaSeconds :type "Float (single-precision)"))
  (`SceneComponent.K2_SetRelativeLocation` (`self.Mesh_Lever`) (`KismetMathLibrary.MakeVector` -10.0 0.0 (- (* (`self.ThrottleVal`) 100.0) 50.0)) false false))

(event `self.Interact_Down`
  (set `self.ThrottleVal` (`KismetMathLibrary.FClamp` (- (`self.ThrottleVal`) (`self.StepAmmount`))))
  (goto _label))

(event `UpdateBoat`
  (bind _asactor_boat (cast `Actor_Boat` (`self.GetParentActor`))))

(fn `UserConstructionScript`)