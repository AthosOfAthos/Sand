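; A sliding door actor on the boat that opens when used and then closes by itself.
; InteractUse sets IsOpening, and Tick eases the door mesh along its local X axis with FInterpTo.
; Near the open position the flag clears, so the door immediately slides back to zero at constant speed through FInterpToConstant, with no hold delay.
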(event `self.Interact_Use`
  (set `self.IsOpening` true))

(event `self.ReceiveTick`
  (params (DeltaSeconds :type "Float (single-precision)"))
  (bind _mesh_door (`self.Mesh_Door`))
  (if (`self.IsOpening`)
    (`SceneComponent.K2_SetRelativeLocation` _mesh_door (`KismetMathLibrary.MakeVector` (`KismetMathLibrary.FInterpTo` (.x (`SceneComponent.RelativeLocation` (`self.Mesh_Door`))) 160.0 (`GameplayStatics.GetWorldDeltaSeconds`) 5.0)) false false)
    (if (> (.x (`SceneComponent.RelativeLocation` (`self.Mesh_Door`))) 150.0)
      (set `self.IsOpening` false))
    (else
      (`SceneComponent.K2_SetRelativeLocation` _mesh_door (`KismetMathLibrary.MakeVector` (`KismetMathLibrary.FInterpTo_Constant` (.x (`SceneComponent.RelativeLocation` (`self.Mesh_Door`))) 0.0 (`GameplayStatics.GetWorldDeltaSeconds`) 100.0)) false false))))

(fn `UserConstructionScript`)